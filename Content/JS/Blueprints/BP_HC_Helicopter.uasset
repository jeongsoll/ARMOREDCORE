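; Enemy helicopter, run by BP_JS_AIController, that targets player 0 and fires aimed bullets at them.
; Each Tick, Sight records front, side or back flags by dot product, while AllShooting passes eight wing arrows to ShootBullet.
; The arrows share one fire timer, bullet count and cooldown, so both timers advance eight times per frame.
; Movement helpers handle acceleration, fixed-altitude flight and pattern-based turning, but nothing here calls them.
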(event `self.ReceiveBeginPlay`
  (cast `/Game/JS/Blueprints/BP_JS_AIController` (`AIBlueprintHelperLibrary.GetAIController` self))
  (set `self.Target` (`GameplayStatics.GetPlayerCharacter` 0))
  (set `self.CurHP` (`self.MaxHP`)))

(event `self.ReceiveTick`
  (params (DeltaSeconds :type "Float (single-precision)"))
  (`self.Sight`)
  (`self.AllShooting` (`self.LArrowComp`) (`self.LArrowComp1`) (`self.LArrowComp2`) (`self.LArrowComp3`) (`self.RArrowComp`) (`self.RArrowComp1`) (`self.RArrowComp2`) (`self.RArrowComp3`) DeltaSeconds))

(fn `Acceleration`
  (bind _returnvalue (+ (`self.CurrentSpeed`) (* (`GameplayStatics.GetWorldDeltaSeconds`) 120.0)))
  (if (>= _returnvalue 600.0)
    (set `self.CurrentSpeed` 600.0)
    (else
      (set `self.CurrentSpeed` _returnvalue))))

(fn `AllShooting`
  (params (LArrowComp :type "SceneComponent Object Reference") (LArrowComp1 :type "SceneComponent Object Reference") (LArrowComp2 :type "SceneComponent Object Reference") (LArrowComp3 :type "SceneComponent Object Reference") (RArrowComp :type "SceneComponent Object Reference") (RArrowComp1 :type "SceneComponent Object Reference") (RArrowComp2 :type "SceneComponent Object Reference") (RArrowComp3 :type "SceneComponent Object Reference") (DeltaSec :type "Float (double-precision)"))
  (`self.ShootBullet` DeltaSec LArrowComp)
  (`self.ShootBullet` DeltaSec LArrowComp1)
  (`self.ShootBullet` DeltaSec LArrowComp2)
  (`self.ShootBullet` DeltaSec LArrowComp3)
  (`self.ShootBullet` DeltaSec RArrowComp)
  (`self.ShootBullet` DeltaSec RArrowComp1)
  (`self.ShootBullet` DeltaSec RArrowComp2)
  (`self.ShootBullet` DeltaSec RArrowComp3))

(fn `FirstPatten`
  (if (`self.bfirstPatten`)
    (bind _output_get (set `self.Direction` (`KismetMathLibrary.Normal` (- (`self.K2_GetActorLocation` (`self.Target`)) (`self.K2_GetActorLocation`)))))
    (bind (_returnvalue_roll _returnvalue_pitch _returnvalue_yaw) (`KismetMathLibrary.BreakRotator` (`KismetMathLibrary.MakeRotFromXZ` _output_get (`self.GetActorUpVector`))))
    (`self.K2_SetActorRotation` (`KismetMathLibrary.MakeRotator` 0.0 -30.0 _returnvalue_yaw))
    (set `self.bfirstPatten` false)
    (else
      (bind _output_get_2 (set `self.Direction` (`self.GetActorForwardVector`)))
      (bind (_returnvalue_roll_2 _returnvalue_pitch_2 _returnvalue_yaw_2) (`KismetMathLibrary.BreakRotator` (`KismetMathLibrary.MakeRotFromXZ` _output_get_2 (`self.GetActorUpVector`))))
      (`self.K2_SetActorRotation` (`KismetMathLibrary.MakeRotator` 0.0 0.0 _returnvalue_yaw_2))
      (set `self.bfirstPatten` true))))

(fn `SetLocation`
  (bind (_returnvalue_x _returnvalue_y) (`KismetMathLibrary.BreakVector` (+ (* (`self.Direction`) (`self.CurrentSpeed`) (`GameplayStatics.GetWorldDeltaSeconds`)) (`self.K2_GetActorLocation`))))
  (`self.K2_SetActorLocation` (`KismetMathLibrary.MakeVector` _returnvalue_x _returnvalue_y 700.0)))

(fn `SetRotation`
  (switch `int` (`self.PattenNum`)
    (:`0`
      (`self.FirstPatten`))
    (:`1`
      (bind _output_get (set `self.Direction` (`KismetMathLibrary.Normal` (- (`self.K2_GetActorLocation` (`self.Target`)) (`self.K2_GetActorLocation`)))))
      (bind (_returnvalue_roll _returnvalue_pitch _returnvalue_yaw) (`KismetMathLibrary.BreakRotator` (`KismetMathLibrary.MakeRotFromXZ` _output_get (`self.GetActorUpVector`))))
      (`self.K2_SetActorRotation` (`KismetMathLibrary.MakeRotator` 0.0 0.0 _returnvalue_yaw)))))

(fn `ShootBullet`
  (params (B :type "Float (double-precision)") (comp :type "SceneComponent Object Reference"))
  (bind (_returnvalue_roll _returnvalue_pitch _returnvalue_yaw) (`KismetMathLibrary.BreakRotator` (`KismetMathLibrary.MakeRotationFromAxes` (`KismetMathLibrary.Normal` (- (`self.K2_GetActorLocation` (`self.Target`)) (`SceneComponent.K2_GetComponentLocation` comp))))))
  ; 0.1초마다 bullet 스폰
  (bind _output_get (set `self.BulletSpawnTime` (+ (`self.BulletSpawnTime`) B)))
  (if (>= _output_get 0.1)
    (if (<= (`self.BulletNum`) 200)
      (`SceneComponent.K2_SetWorldRotation` comp (`KismetMathLibrary.MakeRotator` _returnvalue_roll _returnvalue_pitch _returnvalue_yaw) false false)
      (`|SpawnActorFromClass` "/Game/JS/Blueprints/JS_Bullet.JS_Bullet_C" (`SceneComponent.K2_GetComponentToWorld` comp) "Undefined" "MultiplyWithRoot" null null)
      (set `self.BulletSpawnTime` 0.0)
      (set `self.BulletNum` (+ (`self.BulletNum`) 1))
      (else
        (set `self.BulletCoolTime` (+ (`self.BulletCoolTime`) B))
        (if (>= (`self.BulletCoolTime`) 2.0)
          (set `self.BulletNum` 0)
          (set `self.BulletCoolTime` 0.0))))))

(fn `Sight`
  (bind _returnvalue (`KismetMathLibrary.Dot_VectorVector` (`self.GetActorForwardVector`) (`KismetMathLibrary.Normal` (- (`self.K2_GetActorLocation` (`self.Target`)) (`self.K2_GetActorLocation`)))))
  (bind _returnvalue_2 (> _returnvalue 0.0))
  (bind _returnvalue_3 (== _returnvalue 0.0))
  (bind _returnvalue_4 (< _returnvalue 0.0))
  (if _returnvalue_2
    (set `self.bover` _returnvalue_2)
    (elif _returnvalue_3
      (set `self.bsame` _returnvalue_3)
      (elif _returnvalue_4
        (set `self.bunder` _returnvalue_4)))))

(fn `UserConstructionScript`)