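; Behavior tree service that picks the next attack or action pattern ("Patten") for an AI pawn through its blackboard.
; On each activation, while bFinishPatten is true, it adds frame delta time to a short cooldown, then writes a fixed PattenIndex, clears the flag and resets the timer.
; The writes go through OwnerController, which is set to None, and a random index roll is left unconnected.
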(event `self.ReceiveActivationAI`
  (params (OwnerController :type "AIController Object Reference") (ControlledPawn :type "Pawn Object Reference"))
  (bind _returnvalue (`AIBlueprintHelperLibrary.GetBlackboard` (`self.Owner Controller`)))
  (set `self.Owner Controller` null)
  (if (`BlackboardComponent.GetValueAsBool` (`AIBlueprintHelperLibrary.GetBlackboard` ControlledPawn) "bFinishPatten")
    (bind _output_get (set `self.PattenCoolTime` (+ (`self.PattenCoolTime`) (`GameplayStatics.GetWorldDeltaSeconds`))))
    (if (>= _output_get 0.5)
      (`BlackboardComponent.SetValueAsInt` _returnvalue "PattenIndex" 1)
      (`BlackboardComponent.SetValueAsBool` _returnvalue "bFinishPatten" false)
      (set `self.PattenCoolTime` 0.0))))