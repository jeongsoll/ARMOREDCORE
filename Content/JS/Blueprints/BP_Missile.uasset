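; BP_Missile is a homing missile that targets the player's BP_PlayerMech, with its damage set at BeginPlay.
; Tick first accelerates it along its forward vector up to a speed cap until TargetCheckTime elapses.
; It then turns toward the player each frame, calls FireInDirection and moves by Speed, while the separately ramped ACSpeed is unused in that movement.
; The Life function destroys it after a fixed lifetime.
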(event `self.ReceiveBeginPlay`
  (set `self.Damage` 200.0)
  (bind _asbp_player_mech (cast `/Game/JJH/Blueprints/BP_PlayerMech` (`GameplayStatics.GetPlayerCharacter` 0)))
  (set `self.Player` _asbp_player_mech))

(event `self.ReceiveTick`
  (params (DeltaSeconds :type "Float (single-precision)"))
  (`self.Life`)
  (set `self.JS_CurrentTime` (+ DeltaSeconds (`self.JS_CurrentTime`)))
  (if (>= (`self.JS_CurrentTime`) (`self.TargetCheckTime`))
    (`self.Player`
      (:`then`
        (`self.K2_SetActorRotation` (`KismetMathLibrary.Conv_VectorToRotator` (- (`self.K2_GetActorLocation` (`self.Player`)) (`self.K2_GetActorLocation`))))
        (if (>= (`self.ACSpeed`) 10000.0)
          (set `self.ACSpeed` 10000.0)
          (else
            (set `self.ACSpeed` (+ (`self.ACSpeed`) (* (`GameplayStatics.GetWorldDeltaSeconds`) 600.0)))))
        (bind _output_get (set `self.Direction` (`KismetMathLibrary.Normal` (- (`self.K2_GetActorLocation` (`self.Player`)) (`self.K2_GetActorLocation`)))))
        (`self.FireInDirection` _output_get)
        (`self.K2_SetActorLocation` (+ (* _output_get (`self.Speed`) (`GameplayStatics.GetWorldDeltaSeconds`)) (`self.K2_GetActorLocation`))))
      (:`else`))
    (else
      (if (>= (`self.Speed`) 2000.0)
        (set `self.Speed` 2000.0)
        (else
          (set `self.Speed` (+ (`self.Speed`) (* (`GameplayStatics.GetWorldDeltaSeconds`) 600.0)))))
      (bind _output_get_2 (set `self.Direction` (`self.GetActorForwardVector`)))
      (`self.K2_SetActorLocation` (+ (* (`KismetMathLibrary.Normal` _output_get_2) (`self.Speed`) (`GameplayStatics.GetWorldDeltaSeconds`)) (`self.K2_GetActorLocation`))))))

(fn `Life`
  (bind _output_get (set `self.JS_LifeTime` (+ (`self.JS_LifeTime`) (`GameplayStatics.GetWorldDeltaSeconds`))))
  (if (>= _output_get 13.0)
    (`self.K2_DestroyActor`)
    (else
      (return))))

(fn `UserConstructionScript`)