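; BP_PlayerMech is the player mech Blueprint, which handles the visibility of the booster effects on the mech.
; Every Tick, IsBoostOn shows or hides the left, middle and right boosters, while IsQuickBoostTrigger drives the big middle booster.
; Disconnected debug print nodes for camera, movement, boost gauge and HP values remain in the graph but never run.
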(event `self.ReceiveTick`
  (params (DeltaSeconds :type "Float (single-precision)"))
  (bind _isbooston (`self.IsBoostOn`))
  (`|ExecutionSequence`
    (:`then_0`
      (`SceneComponent.SetVisibility` (`self.BoosterLeft`) _isbooston false))
    (:`then_1`
      (`SceneComponent.SetVisibility` (`self.BoosterMiddle`) _isbooston false))
    (:`then_2`
      (`SceneComponent.SetVisibility` (`self.BoosterRight`) _isbooston false))
    (:`then_3`
      (`SceneComponent.SetVisibility` (`self.BigBoosterMiddle`) (`self.IsQuickBoostTrigger`) false))))

(fn `UserConstructionScript`)